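; Base arrow item that plugs into the owner's equipment component as the equipped ammunition.
; Using it passes itself to BPC_Equipment's UpdateArrows to equip or unequip it.
; Dropping it runs the parent logic, then clears the arrows slot if this item occupies it.
; GetArrowInfo looks up the arrow's data in DT_Arrows, using ItemId as the row name.
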(event EventUseItem
  (bind _returnvalue (Components|GetOwner))
  (bind _returnvalue_2 (Actor|GetComponentbyClass _returnvalue "/Game/DynamicCombatSystem/Blueprints/Components/BPC_Equipment.BPC_Equipment_C"))
  ;[0.2048 0.4427 0.1272] Equip/Unequip item on use
  (Utilities|IsValid _returnvalue_2
    (:Is%20Valid
      (Default|UpdateArrows _returnvalue_2 self))))

(event EventDropItem
  (params (Count :type Integer))
  (bind _returnvalue (Components|GetOwner))
  (bind _returnvalue_2 (Actor|GetComponentbyClass _returnvalue "/Game/DynamicCombatSystem/Blueprints/Components/BPC_Equipment.BPC_Equipment_C"))
  ;[0.2048 0.4427 0.1272] Remove arrows  from equipment component if it was already used
  (|CallParentFunction Count)
  (Utilities|IsValid _returnvalue
    (:Is%20Valid
      (Utilities|IsValid _returnvalue_2
        (:Is%20Valid
          (if (== (Variables|/Game/DynamicCombatSystem/Blueprints/Components/BPC_Equipment.BPC_Equipment_C|GetArrowsSlot _returnvalue_2) self)
            (Default|UpdateArrows _returnvalue_2)))))))

(fn ConstructionScript
  (|CallParentFunction))

(fn GetArrowInfo
  (bind _returnvalue (Utilities|GetDataTableRow "/Game/DynamicCombatSystem/DataTables/DT_Arrows.DT_Arrows" (Variables|Default|GetItemId))
    (:then
      (return _returnvalue))
    (:RowNotFound
      (return ""))))