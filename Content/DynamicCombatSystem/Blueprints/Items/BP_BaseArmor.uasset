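; BP_BaseArmor is the base armor item of the combat system, which owners equip or unequip through their BPC_Equipment component.
; GetArmorInfo reads the item's row from DT_Armor by ItemId to supply the armor type.
; Using the item passes it and its type to UpdateArmor.
; Dropping it calls the parent logic, then makes the same call if the item still occupies that armor slot, removing it from equipment.
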(event EventBeginPlay
  (|CallParentFunction))

(event EventDropItem
  (params (Count :type Integer))
  (bind _returnvalue (Components|GetOwner))
  (bind _returnvalue_2 (Actor|GetComponentbyClass _returnvalue "/Game/DynamicCombatSystem/Blueprints/Components/BPC_Equipment.BPC_Equipment_C"))
  ;[1 1 1] Remove armor from equipment component if it was already used
  (|CallParentFunction Count)
  (Utilities|IsValid _returnvalue
    (:Is%20Valid
      (Utilities|IsValid _returnvalue_2
        (:Is%20Valid
          (if (== (Default|GetArmorItem _returnvalue_2 (.Type (Utilities|Struct|BreakF_Armor (CallFunction|GetArmorInfo)))) self)
            (Default|UpdateArmor _returnvalue_2 self (.Type (Utilities|Struct|BreakF_Armor (CallFunction|GetArmorInfo))))))))))

(event EventUseItem
  (bind _returnvalue (Components|GetOwner))
  (bind _returnvalue_2 (Actor|GetComponentbyClass _returnvalue "/Game/DynamicCombatSystem/Blueprints/Components/BPC_Equipment.BPC_Equipment_C"))
  ;[1 1 1] Equip/Unequip item on use
  (Utilities|IsValid _returnvalue_2
    (:Is%20Valid
      (Default|UpdateArmor _returnvalue_2 self (.Type (Utilities|Struct|BreakF_Armor (CallFunction|GetArmorInfo)))))))

(fn ConstructionScript
  (|CallParentFunction))

(fn GetArmorInfo
  (bind _returnvalue (Utilities|GetDataTableRow "/Game/DynamicCombatSystem/DataTables/DT_Armor.DT_Armor" (Variables|Default|GetItemId))
    (:then
      (return _returnvalue))
    (:RowNotFound
      (return ""))))