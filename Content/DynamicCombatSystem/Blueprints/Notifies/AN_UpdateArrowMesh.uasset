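; AN_UpdateArrowMesh is an animation notify that updates the arrow mesh on a bow-using character at a chosen animation frame.
; On firing, it casts the mesh owner to BP_CombatCharacter, falling back to BP_ArcherAI for enemy archers.
; It then calls that actor's UpdateArrowMesh, passing the notify's Visible and AttachToHand settings to control visibility and hand attachment.
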(fn ReceivedNotify
  (params (MeshComp :type Skeletal%20Mesh%20Component%20Object%20Reference) (Animation :type Anim%20Sequence%20Base%20Object%20Reference))
  (bind _returnvalue (Components|GetOwner MeshComp))
  (Utilities|IsValid _returnvalue
    (:Is%20Valid
      (bind _asbp_combat_character (Utilities|Casting|CastToBP_CombatCharacter _returnvalue)
        (:then
          (Default|UpdateArrowMesh _asbp_combat_character (Variables|Default|GetVisible) (Variables|Default|GetAttachToHand)))
        (:CastFailed
          ;[0.2048 0.4427 0.1272] If called by Archer AI
          (bind _asbp_archer_ai (Utilities|Casting|CastToBP_ArcherAI _returnvalue))
          (Default|UpdateArrowMesh _asbp_archer_ai (Variables|Default|GetVisible) (Variables|Default|GetAttachToHand))))
      (return false))))

(fn GetNotifyName
  (return "UpdateArrowMesh"))