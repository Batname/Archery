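; Arrow projectile for the combat system that damages what it hits and leaves an impaled arrow attached to the struck bone.
; A spawn-set speed alpha scales launch speed, damage and physics impulse, and gravity is set after a short delay.
; Sphere overlap triggers a forward trace to find the mesh bone instead of the capsule, enabling headshot multipliers.
; Owners with a behavior component only hit attackable targets listed as enemies.
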(event OnComponentBeginOverlap(Sphere)
  (params (OverlappedComponent :type Primitive%20Component%20Object%20Reference) (OtherActor :type Actor%20Object%20Reference) (OtherComp :type Primitive%20Component%20Object%20Reference) (OtherBodyIndex :type Integer) (bFromSweep :type Boolean) (SweepResult :type Hit%20Result%20Structure%20%28by%20ref%29))
  (bind _sphere (Variables|Default|GetSphere))
  (bind _damage (Variables|Default|GetDamage))
  (bind _initialspeedalpha (Variables|Default|GetInitialSpeedAlpha))
  (bind _returnvalue (Transformation|GetWorldLocation _sphere))
  (bind _returnvalue_2 (* _damage _initialspeedalpha))
  ;[0.2048 0.4427 0.1272] Make sure overlapped actor was not the owner
  (if (!= (Components|GetOwner) OtherActor)
    (Utilities|FlowControl|DoOnce false
      (:Completed
        ;[0.2048 0.4427 0.1272] Do the line trace test to find character's mesh instead of capsule
        (bind (_outhit _returnvalue_3) (Collision|SphereTraceByChannel _returnvalue (+ _returnvalue (* (Math|Vector|GetForwardVector (Transformation|GetWorldRotation _sphere)) 1e+02)) 1.0 "TraceTypeQuery3" false 0 "None"))
        (if _returnvalue_3
          (if (and (!= (Components|GetOwner) (.HitActor (Collision|BreakHitResult _outhit))) (CallFunction|IsEnemy (.HitActor (Collision|BreakHitResult _outhit))))
            (bind _socketname (Class|BPIIsAttackable|GetHeadSocket(Message) (.HitActor (Collision|BreakHitResult _outhit))))
            ;[0.2048 0.4427 0.1272] Apply Damage
            (Class|BPIIsAttackable|HandleHit(Message) (.HitActor (Collision|BreakHitResult _outhit)) (select (Utilities|Name|Equal(Name) _socketname (.HitBoneName (Collision|BreakHitResult _outhit))) (* _returnvalue_2 (Variables|Default|GetHeadShotDamageMultiplier)) _returnvalue_2) "NewEnumerator14" "NewEnumerator6" (Components|GetOwner) (Variables|Default|GetWasCritical))
            ;[0.2048 0.4427 0.1272] Spawn and attach Impaled Arrow to hit bone
            (Components|Movement|StopMovementImmediately (Variables|Default|GetProjectileMovement))
            (bind _returnvalue_4 (Game|SpawnActorfromClass "/Game/DynamicCombatSystem/Blueprints/Projectiles/BP_ImpaledArrow.BP_ImpaledArrow_C" (Math|Transform|MakeTransform (.Location (Collision|BreakHitResult _outhit)) (Transformation|GetActorRotation) (Transformation|GetActorScale3D)) "AlwaysSpawn" (.HitActor (Collision|BreakHitResult _outhit)) (Variables|Default|GetArrowMesh) (Game|GetInstigator (Components|GetOwner))))
            (Transformation|AttachComponentToComponent _returnvalue_4 (.HitComponent (Collision|BreakHitResult _outhit)) (.HitBoneName (Collision|BreakHitResult _outhit)) "KeepWorld" "KeepWorld" "KeepWorld" true)
            ;[0.2048 0.4427 0.1272] Apply impulse if target has physics enabled
            (CallFunction|ApplyImpulse (.HitComponent (Collision|BreakHitResult _outhit)) (.Normal (Collision|BreakHitResult _outhit)) (.HitBoneName (Collision|BreakHitResult _outhit)))
            (Actor|DestroyActor)
            (else
              (CallFunction|ResetTraceTest :!label _label)))
          (else
            (goto _label)))))))

(event Custom|ResetTraceTest
  (bind _sphere (Variables|Default|GetSphere))
  (bind _damage (Variables|Default|GetDamage))
  (bind _initialspeedalpha (Variables|Default|GetInitialSpeedAlpha))
  (bind _returnvalue (Transformation|GetWorldLocation _sphere))
  (bind _returnvalue_2 (* _damage _initialspeedalpha))
  (Utilities|FlowControl|DoOnce false) ; enters at Reset
)

(event EventBeginPlay
  (bind _projectilemovement (Variables|Default|GetProjectileMovement))
  ;[0.2048 0.4427 0.1272] Set InitialSpeed based on alpha set on spawn
  (Variables|/Script/Engine.ProjectileMovementComponent|SetInitialSpeed _projectilemovement (* (Variables|/Script/Engine.ProjectileMovementComponent|GetInitialSpeed _projectilemovement) (Variables|Default|GetInitialSpeedAlpha)))
  (Components|StaticMesh|SetStaticMesh (Variables|Default|GetStaticMesh) (Variables|Default|GetArrowMesh))
  (Actor|SetLifeSpan (Variables|Default|GetLifeTime))
  (Utilities|FlowControl|Delay 0.3)
  (Variables|/Script/Engine.ProjectileMovementComponent|SetProjectileGravityScale (Variables|Default|GetProjectileMovement) 0.3))

(fn ConstructionScript)

(fn ApplyImpulse
  (params (Component :type Primitive%20Component%20Object%20Reference) (HitNormal :type Vector) (BoneName :type Name))
  (if (Class|SceneComponent|IsAnySimulatingPhysics Component)
    (Physics|AddImpulse Component (* (* HitNormal -1.0) (* (Variables|Default|GetInitialSpeedAlpha) 1e+04)) BoneName false)))

(fn IsEnemy
  (params (Target :type Actor%20Object%20Reference))
  (bind _returnvalue (Components|GetOwner))
  (bind _returnvalue_2 (Actor|GetComponentbyClass _returnvalue "/Game/DynamicCombatSystem/Blueprints/Components/BPC_Behavior.BPC_Behavior_C"))
  ;[0.2048 0.4427 0.1272] If Owner has BehaviorComponent, make sure attacked actor is his enemy
  (if (Utilities|DoesObjectImplementInterface Target "/Game/DynamicCombatSystem/Blueprints/Interfaces/BPI_IsAttackable.BPI_IsAttackable_C")
    (Utilities|IsValid _returnvalue_2
      (:Is%20Valid
        (return (Utilities|Array|ContainsItem (Variables|/Game/DynamicCombatSystem/Blueprints/Components/BPC_Behavior.BPC_Behavior_C|GetEnemies _returnvalue_2) (Utilities|GetClass Target))))
      (:Is%20Not%20Valid
        _)))
  (return true))