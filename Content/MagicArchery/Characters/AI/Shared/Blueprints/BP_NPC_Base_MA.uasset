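; BP_NPC_Base_MA is a base NPC Blueprint for Magic Archery that displays the character's health as text.
; UpdateHPText converts Health to text and writes it to the HPTextRender component.
; It runs on BeginPlay after the parent's logic and again every Tick, a per-frame refresh marked as temporary.
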(event EventBeginPlay
  ;[1 1 1] Comment
  (|CallParentFunction)
  (CallFunction|UpdateHPText))

(event Collision|EventActorBeginOverlap
  (params (OtherActor :type Actor%20Object%20Reference)))

(event EventTick
  (params (DeltaSeconds :type Float%20%28single-precision%29))
  ;[1 1 1] TEMP
  (CallFunction|UpdateHPText))

(fn ConstructionScript
  (|CallParentFunction))

(fn UpdateHPText
  (Rendering|Components|TextRender|SetText (Variables|Default|GetHPTextRender) (Utilities|Text|ToText(Float) (Variables|Default|GetHealth) "HalfToEven")))