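; BP_AIComponent_Base_Target is an AI component that sets up blackboard and behavior tree logic for its owning character.
; On BeginPlay, SetDefaults gets the owner's AI controller and caches it along with its controlled Character.
; If a blackboard asset is set, the controller initializes it and the component stores the blackboard component.
; The behavior tree runs only when both that asset and a tree are valid.
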(event EventBeginPlay
  (CallFunction|SetDefaults))

(fn SetDefaults
  (bind _returnvalue (Components|GetOwner))
  (bind _behaviortreeref (Variables|Default|GetBehaviorTreeRef))
  (bind _blackboardasset (Variables|Default|GetBlackboardAsset))
  (bind _returnvalue_2 (AI|GetAIController _returnvalue))
  ;[1 1 1] Comment
  (Utilities|IsValid _returnvalue_2
    (:Is%20Valid
      (bind _output_get (Variables|Default|SetAIController_Ref _returnvalue_2))
      (bind _ascharacter (Utilities|Casting|CastToCharacter (Pawn|GetControlledPawn _output_get)))
      (Variables|Default|SetAICharacterRef _ascharacter)
      (Utilities|IsValid _blackboardasset
        (:Is%20Valid
          (bind _blackboardcomponent (Class|AIController|UseBlackboard _returnvalue_2 _blackboardasset))
          (Variables|Default|SetBlackboardComonent _blackboardcomponent)
          (Utilities|IsValid _behaviortreeref
            (:Is%20Valid
              (AI|RunBehaviorTree _returnvalue_2 _behaviortreeref))))))))