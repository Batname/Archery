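; Magic Leap meshing actor for the archery game that sets up world meshing and spawns test or gameplay NPCs.
; On BeginPlay it connects MeshTracker to the MRMesh, skipping dedicated servers, and enables player input.
; Either Home button or the 2 key alternately spawns an archer or civilian along the XR camera's forward vector.
; Pushing the right thumbstick Z axis near maximum destroys all BP_NPC_Base actors.
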(event EventBeginPlay
  (Utilities|FlowControl|Sequence
    (:then_0
      (Networking|SwitchHasAuthority
        (:Authority
          ;[1 1 1] Not Dedicated server
          (if (not (Networking|IsDedicatedServer))
            ;[1 1 1] Client Execution only
            (CallFunction|InitMagicLeap :!label _label)))
        (:Remote
          (goto _label))))
    (:then_1
      (Input|EnableInput (Game|GetPlayerController 0)))))

(event Input|KeyboardEvents|MotionControllerRightThumbstickZ
  (params (AxisValue :type Float%20%28single-precision%29))
  ;[1 1 1] Delete all AI
  (if (>= AxisValue 0.9)
    (bind _outactors (Actor|GetAllActorsOfClass "/Game/AIBehaviorToolkit/Blueprints/BP_NPC_Base.BP_NPC_Base_C"))
    (for _array_element _outactors
      (Actor|DestroyActor _array_element))))

(event Input|KeyboardEvents|2
  (params (Key :type Key%20Structure))
  ;[1 1 1] Spawn AI
  (:Pressed
    (if (Variables|Default|GetbIsArcherySpawn)
      (CallFunction|SpawnCharacter "/Game/MagicArchery/Characters/AI/Archer/Blueprints/BP_Archer_MA.BP_Archer_MA_C" 1e+02 true 0.2)
      (Variables|Default|SetbIsArcherySpawn false)
      (else
        (CallFunction|SpawnCharacter "/Game/MagicArchery/Characters/AI/Civilian/Blueprints/BP_NPC_Civilian_MA.BP_NPC_Civilian_MA_C" 1e+02 true 0.2)
        (Variables|Default|SetbIsArcherySpawn true)))))

(event Input|KeyboardEvents|MagicLeapLeftHomeButton
  (params (Key :type Key%20Structure))
  ;[1 1 1] Spawn AI
  (:Pressed
    (if (Variables|Default|GetbIsArcherySpawn)
      (CallFunction|SpawnCharacter "/Game/MagicArchery/Characters/AI/Archer/Blueprints/BP_Archer_MA.BP_Archer_MA_C" 1e+02 true 0.2)
      (Variables|Default|SetbIsArcherySpawn false)
      (else
        (CallFunction|SpawnCharacter "/Game/MagicArchery/Characters/AI/Civilian/Blueprints/BP_NPC_Civilian_MA.BP_NPC_Civilian_MA_C" 1e+02 true 0.2)
        (Variables|Default|SetbIsArcherySpawn true)))))

(event Input|KeyboardEvents|MagicLeapRightHomeButton
  (params (Key :type Key%20Structure))
  ;[1 1 1] Spawn AI
  (:Pressed
    (if (Variables|Default|GetbIsArcherySpawn)
      (CallFunction|SpawnCharacter "/Game/MagicArchery/Characters/AI/Archer/Blueprints/BP_Archer_MA.BP_Archer_MA_C" 1e+02 true 0.2)
      (Variables|Default|SetbIsArcherySpawn false)
      (else
        (CallFunction|SpawnCharacter "/Game/MagicArchery/Characters/AI/Civilian/Blueprints/BP_NPC_Civilian_MA.BP_NPC_Civilian_MA_C" 1e+02 true 0.2)
        (Variables|Default|SetbIsArcherySpawn true)))))

(fn ConstructionScript)

(fn InitMagicLeap
  (Class|MeshTrackerComponent|ConnectMRMesh (Variables|Default|GetMeshTracker) (Variables|Default|GetMRMesh)))

(fn SpawnCharacter
  (params (Class :type Actor%20Class%20Reference) (Distance :type Float%20%28single-precision%29) (bIsDebug :type Boolean) (Scale :type Float%20%28single-precision%29))
  (bind _asbp_archery_pawn (Utilities|Casting|CastToBP_Archery_Pawn (Game|Player|GetPlayerPawn 0)))
  (Development|PrintString (Utilities|String|ToString(Vector) (+ (Transformation|GetWorldLocation (Variables|/Game/MagicArchery/CoreBPs/BP_Archery_Pawn.BP_Archery_Pawn_C|GetXR_Camera _asbp_archery_pawn)) (* (Math|Vector|GetForwardVector (Variables|/Game/MagicArchery/CoreBPs/BP_Archery_Pawn.BP_Archery_Pawn_C|GetXR_Camera _asbp_archery_pawn)) Distance))) bIsDebug bIsDebug)
  (Game|SpawnActorfromClass Class (Math|Transform|MakeTransform (+ (Transformation|GetWorldLocation (Variables|/Game/MagicArchery/CoreBPs/BP_Archery_Pawn.BP_Archery_Pawn_C|GetXR_Camera _asbp_archery_pawn)) (* (Math|Vector|GetForwardVector (Variables|/Game/MagicArchery/CoreBPs/BP_Archery_Pawn.BP_Archery_Pawn_C|GetXR_Camera _asbp_archery_pawn)) Distance)) "0, 0, 0" (Math|Conversions|ToVector(Float) Scale)) "AlwaysSpawn" 0 0))